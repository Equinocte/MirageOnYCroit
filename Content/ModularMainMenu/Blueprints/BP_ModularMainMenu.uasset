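; Modular main menu manager actor that opens and closes the menu widget as either a start or in-game pause menu.
; BeginPlay loads saved namespaces, spawns an input manager, seeds first-run default settings, runs graphics and console commands, then routes by IsInGame.
; Tick polls activation keys for a debounced toggle.
; Showing applies pause-policy time dilation; hiding restores time, reverses the opening animation and restores mobile touch controls on touch platforms.
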(event Custom|CloseMenu
  ;[0.9793 0.4828 1] SHOW/HIDE MENU
  (Variables|Default|SetIsMenuOpen? false)
  (CallFunction|HideMainMenu))

(event Custom|ShowMainMenu
  ;[0.5038 1 0.5785] SHOW MENU
  (Input|EnableInput (Variables|Default|GetinputManager) (Game|GetPlayerController 0))
  (Variables|Default|SetIsMenuOpen? true)
  (if (Variables|Menu|GetisInGame)
    (Utilities|Time|SetGlobalTimeDilation (Utilities|Select :Index (Variables|Menu|GetGamePausePolicy) :NewEnumerator0 1.0 :NewEnumerator1 0.5 :NewEnumerator3 0.25 :NewEnumerator2 1e-06))
    (else
      (Utilities|Time|SetGlobalTimeDilation 1.0)))
  (bind _returnvalue (UserInterface|CreateWidget "/Game/ModularMainMenu/Misc/Menu/WB_MenuWidget.WB_MenuWidget_C" (Game|GetPlayerController 0)))
  (Variables|/Game/ModularMainMenu/Misc/Menu/WB_MenuWidget.WB_MenuWidget_C|SetgameInfo _returnvalue (Utilities|Struct|MakeSTR_GameInfo (Variables|GameInfo|GetGameTitle) (Variables|GameInfo|GetVersion) (Variables|GameInfo|GetDevelopers) (Variables|GameInfo|GetshowPlayerName)))
  (Input|SetInputModeGameandUI (Game|GetPlayerController 0) _returnvalue "DoNotLock" true)
  (bind _output_get (Variables|Default|Setwidget _returnvalue))
  (Variables|/Game/ModularMainMenu/Misc/BP_InputManager.BP_InputManager_C|SetWidget (Variables|Default|GetinputManager) _output_get)
  (UserInterface|Viewport|AddtoViewport _returnvalue 9999)
  (Variables|/Script/Engine.PlayerController|SetbShowMouseCursor (Game|GetPlayerController 0) true)
  (if (Variables|Menu|GetisInGame)
    (Default|UpdatePage (Variables|Default|Getwidget) (Utilities|String|ToString(Name) (Variables|DataSource|GetinGameMenuPage)))
    (else
      (Default|UpdatePage (Variables|Default|Getwidget) (Utilities|String|ToString(Name) (Variables|DataSource|GetStart%20Menu%20Page))))))

(event Custom|HideMainMenu
  (bind _returnvalue (Game|GetPlayerController 0))
  (bind _widget (Variables|Default|Getwidget))
  ;[1 0.2299 0.6301] HIDE MENU
  (Utilities|Time|SetGlobalTimeDilation 1.0) ; Continue the game when menu is hidden or closed
  (Input|DisableInput (Variables|Default|GetinputManager) (Game|GetPlayerController 0)) ; Disable menu input
  (UserInterface|Animation|PlayAnimation (Variables|Default|Getwidget) (Utilities|Select :Index (Variables|Animations|GetMenuOpenAnimation) :NewEnumerator0 (Variables|/Game/ModularMainMenu/Misc/Menu/WB_MenuWidget.WB_MenuWidget_C|GetstartInstant _widget) :NewEnumerator1 (Variables|/Game/ModularMainMenu/Misc/Menu/WB_MenuWidget.WB_MenuWidget_C|GetstartSlide _widget) :NewEnumerator2 (Variables|/Game/ModularMainMenu/Misc/Menu/WB_MenuWidget.WB_MenuWidget_C|GetstartFade _widget) :NewEnumerator4 (Variables|/Game/ModularMainMenu/Misc/Menu/WB_MenuWidget.WB_MenuWidget_C|GetstartStairs _widget)) 0.0 1 "Reverse" 1.0 false) ; Play reversed menu appearance animation
  (Input|SetInputModeGameOnly _returnvalue) ; Hides menu cursor
  (Variables|/Script/Engine.PlayerController|SetbShowMouseCursor _returnvalue false)
  (Utilities|FlowControl|Delay (Utilities|Select :Index (Variables|Animations|GetMenuOpenAnimation) :NewEnumerator0 0.0 :NewEnumerator1 0.5 :NewEnumerator2 0.5 :NewEnumerator4 0.0))
  (Widget|RemovefromParent (Variables|Default|Getwidget)) ; Remove menu widget from the screen
  (CallFunction|ShowMobileInterface))

(event Custom|ToogleMenu
  ;[0.9793 0.4828 1] SHOW/HIDE MENU
  (|SetInputDelay
    (:Return
      (if (Variables|Menu|GetisInGame)
        (if (Variables|Default|GetIsMenuOpen?)
          (Audio|PlaySound2D "/Game/ModularMainMenu/Audio/S_MenuHide.S_MenuHide" 1.0 1.0 0.0 0 0)
          (Variables|Default|SetIsMenuOpen? false)
          (CallFunction|HideMainMenu)
          (else
            (Audio|PlaySound2D "/Game/ModularMainMenu/Audio/S_MenuShow.S_MenuShow" 1.0 1.0 0.0 0 0)
            (if (Variables|Menu|GetEnable%20Menu)
              (Variables|Default|SetIsMenuOpen? true)
              (CallFunction|ShowMainMenu))))))))

(event Custom|OpenMenu
  ;[0.9793 0.4828 1] SHOW/HIDE MENU
  (if (Variables|Menu|GetEnable%20Menu)
    (Variables|Default|SetIsMenuOpen? true)
    (CallFunction|ShowMainMenu)))

(event Custom|HideMobileInterface
  ;[0.3321 0.3618 1] MOBILE TOUCH CONTROLLS
  (if (and (Utilities|Enum|Equal(Enum) (Variables|ControlIdiom|GetIdiom) "NewEnumerator1") (Variables|Menu|GetisInGame))
    (Class|PlayerController|ActivateTouchInterface (Game|GetPlayerController 0))
    (Widget|RemovefromParent (stale Custom|ShowMobileInterface _returnvalue_2))))

(event Custom|ShowMobileInterface
  (bind _returnvalue (Game|GetPlayerController 0))
  ;[0.3321 0.3618 1] MOBILE TOUCH CONTROLLS
  (if (and (Utilities|Enum|Equal(Enum) (Variables|ControlIdiom|GetIdiom) "NewEnumerator1") (Variables|Menu|GetisInGame))
    (Class|PlayerController|ActivateTouchInterface _returnvalue (Variables|Mobile|GetMobileTouchInterface))
    (bind _returnvalue_2 (UserInterface|CreateWidget "/Game/ModularMainMenu/Misc/Mobile/WB_MobileMenuButton.WB_MobileMenuButton_C" _returnvalue))
    (UserInterface|Viewport|AddtoViewport _returnvalue_2 9998)))

(event EventBeginPlay
  (bind _returnvalue (Game|GetPlayerController 0))
  (bind _returnvalue_2 (Game|GetPlayerController 0))
  (bind _default_settings (Variables|DefaultSettings|GetDefault%20Settings))
  ;[1 1 1] Load Saves
  (SaveGame|CreateSaveGameObject "/Game/ModularMainMenu/Misc/BP_NamespaceSerialisation.BP_NamespaceSerialisation_C")
  (bind _returnvalue_3 (SaveGame|LoadGamefromSlot "saved_namespace"))
  (bind _asbp_namespace_serialisation (Utilities|Casting|CastToBP_NamespaceSerialisation _returnvalue_3)
    (:then
      (Variables|Default|SetglobalNamespaces (Variables|/Game/ModularMainMenu/Misc/BP_NamespaceSerialisation.BP_NamespaceSerialisation_C|GetNamespaceArray _asbp_namespace_serialisation)))
    (:CastFailed
      _))
  ;[1 1 1] CREATE INPUT MANAGER INSTANCE
  (bind _returnvalue_4 (Game|SpawnActorfromClass "/Game/ModularMainMenu/Misc/BP_InputManager.BP_InputManager_C" (Math|Transform|MakeTransform "0, 0, 0") "AlwaysSpawn" 0 0))
  (Variables|Default|SetinputManager _returnvalue_4)
  (Utilities|FlowControl|Sequence
    (:then_0
      ;[0.3005 1 0.7286] SET DEFAULT SETTINGS
      (bind _boolean (CallFunction|GetMenuBoolean "is_not_first"))
      (if (not _boolean)
        (bind _keys (Utilities|Map|Keys _default_settings))
        (for _array_element _keys
          (CallFunction|SetMenuString _array_element (.Value (Utilities|Map|Find _default_settings _array_element))))
        (CallFunction|SetMenuBoolean "is_not_first" true)))
    (:then_1
      ;[0.4071 0.3711 1] EXECUTE CONSOLE COMMANDS ON START
      (CallFunction|CustomAction "UpdateGraphics")
      (CallFunction|CustomAction "UpdateVideo")
      (for _array_element_2 (Variables|ConsoleCommandsOverride|GetOverride%20Console%20Commands)
        (Development|ExecuteConsoleCommand _array_element_2 _returnvalue_2))
      (Input|EnableInput _returnvalue_2))
    (:then_2
      ;[1 1 1] ROUTE TO MENU ON START
      (if (Variables|Menu|GetEnable%20Menu)
        (if (Variables|Menu|GetisInGame)
          (Variables|/Script/Engine.PlayerController|SetbShowMouseCursor _returnvalue false)
          (Input|SetInputModeGameOnly _returnvalue)
          (CallFunction|ShowMobileInterface)
          (else
            (CallFunction|ShowMainMenu)))))))

(event EventTick
  (params (DeltaSeconds :type Float%20%28single-precision%29))
  (bind _returnvalue (Game|GetPlayerController 0))
  ;[1 0.8496 0.4547] REGISTER INPUT
  (if (Math|Boolean|ORBoolean (Game|Player|IsInputKeyDown _returnvalue (Variables|Controls|GetPrimaryActivationKey)) (Game|Player|IsInputKeyDown _returnvalue (Variables|Controls|GetSecondaryActivationKey)) (Game|Player|IsInputKeyDown _returnvalue (Variables|Controls|GetTertiaryActivationKey)))
    (Utilities|FlowControl|DoOnce false :!label _label
      (:Completed
        (CallFunction|ToogleMenu)))
    (else
      (goto _label Reset))))

(fn ConstructionScript)

(fn GetAppearance
  (switch Utilities|FlowControl|Switch|SwitchonENUM_InterfaceControlIdiom (Variables|ControlIdiom|GetIdiom)
    (:NewEnumerator0
      (return ""))
    (:NewEnumerator1
      (return ""))))

(fn GetMacro
  (params (For :type String))
  (bind _returnvalue (Utilities|String|Replace For "#"))
  (if (Utilities|String|Contains For "#")
    (bind _array_element (Utilities|Array|ForEachLoopwithBreak (Variables|LevelQniqueMacros|GetMacros) :!label _label)
      (:LoopBody
        (if (Utilities|String|Contains _array_element _returnvalue)
          (Utilities|FlowControl|Sequence
            (:then_0
              (goto _label Break))
            (:then_1
              (if (.ReturnValue (Utilities|String|Split _array_element "="))
                (return (.RightS (Utilities|String|Split _array_element "=")))
                (else
                  (CallFunction|PrintMenuError (Utilities|String|Append "Unresognized macro " _returnvalue))
                  (return For))))))))
    (else
      (return For))))