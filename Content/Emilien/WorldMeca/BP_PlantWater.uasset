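; BP_PlantWater is a world actor that marks a plant interaction zone for the player character, apparently for watering.
; Entering its Sphere creates and shows a WDG_plant widget and sets OnPlantRange on the BP_ThirdPersonCharacter found via GetActorOfClass.
; Leaving hides the widget and clears the flag, printing the value both times.
; Overlaps do not check the other actor, and each entry creates a new widget.
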(event OnComponentBeginOverlap(Sphere)
  (params (OverlappedComponent :type Primitive%20Component%20Object%20Reference) (OtherActor :type Actor%20Object%20Reference) (OtherComp :type Primitive%20Component%20Object%20Reference) (OtherBodyIndex :type Integer) (bFromSweep :type Boolean) (SweepResult :type Hit%20Result%20Structure%20%28by%20ref%29))
  (bind _returnvalue (UserInterface|CreateWidget "/Game/Emilien/WorldMeca/WDG_plant.WDG_plant_C"))
  (bind _output_get (Variables|Default|SetWDG_Plant _returnvalue))
  (UserInterface|Viewport|AddtoViewport _output_get 0)
  (bind _returnvalue_2 (Actor|GetActorOfClass "/Game/ThirdPerson/Blueprints/BP_ThirdPersonCharacter.BP_ThirdPersonCharacter_C"))
  (bind _output_get_2 (Variables|Default|SetRefCharacter _returnvalue_2))
  (bind _output_get_3 (Variables|/Game/ThirdPerson/Blueprints/BP_ThirdPersonCharacter.BP_ThirdPersonCharacter_C|SetOnPlantRange _output_get_2 true))
  (Development|PrintString (Utilities|String|ToString(Boolean) _output_get_3)))

(event OnComponentEndOverlap(Sphere)
  (params (OverlappedComponent :type Primitive%20Component%20Object%20Reference) (OtherActor :type Actor%20Object%20Reference) (OtherComp :type Primitive%20Component%20Object%20Reference) (OtherBodyIndex :type Integer))
  (Widget|SetVisibility (Variables|Default|GetWDG_Plant) "Hidden")
  (bind _output_get (Variables|/Game/ThirdPerson/Blueprints/BP_ThirdPersonCharacter.BP_ThirdPersonCharacter_C|SetOnPlantRange (Variables|Default|GetRefCharacter) false))
  (Development|PrintString (Utilities|String|ToString(Boolean) _output_get)))

(event EventBeginPlay)

(event Collision|EventActorBeginOverlap
  (params (OtherActor :type Actor%20Object%20Reference)))

(fn ConstructionScript)