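; Tornado actor that travels along a spline path placed in the level.
; On BeginPlay it finds a BP_SplinePathTornado actor and starts a timeline, with play rate set from TimeToCompleteInSeconds.
; Each update maps the timeline track to a distance along the spline and moves the actor to that world location.
; Spline rotation is left unused, so the tornado does not turn to follow the path.
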(event Custom|Move_object
  (Components|Timeline|SetPlayRate (Variables|Default|GetMoveObjectTimeLine) (/ 1.0 (Variables|Default|GetTimeToComplete%20%28in%20seconds%29)))
  (bind _movetrack (Timeline|MoveObjectTimeLine Play)
    (:Update
      (Transformation|SetActorTransform (Math|Transform|MakeTransform (Spline|GetLocationatDistanceAlongSpline (Variables|/Game/Tom/FX/Tornado/BP_SplinePathTornado.BP_SplinePathTornado_C|GetSpline (Variables|Default|GetSplineRef)) (Math|Float|Lerp 0.0 (Spline|GetSplineLength (Variables|/Game/Tom/FX/Tornado/BP_SplinePathTornado.BP_SplinePathTornado_C|GetSpline (Variables|Default|GetSplineRef))) _movetrack) "World") "0, 0, 0" "1.000000,1.000000,1.000000")))))

(event EventBeginPlay
  (bind _returnvalue (Actor|GetActorOfClass "/Game/Tom/FX/Tornado/BP_SplinePathTornado.BP_SplinePathTornado_C"))
  (Variables|Default|SetSplineRef _returnvalue)
  (CallFunction|MoveObject))

(fn ConstructionScript)